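; BP_BishopObstacle is a networked obstacle that sends a ragdoll message to any actor overlapping its Box.
; BeginPlay caches the start transform, and Tick passes delta seconds through Move and server-named events into RunningTime2.
; Its RepNotify offsets Y from the start by a sine of RunningTime, which nothing shown updates.
; A second RepNotify applies ActorTransform's location with a debug print.
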(event `self.ReceiveBeginPlay`
  (`self.SRV`))

(event `SRV`
  (set `self.StartTransform` (`self.GetTransform`)))

(event `self.ReceiveTick`
  (params (DeltaSeconds :type "Float (single-precision)"))
  (`self.Move` DeltaSeconds))

(event `Move`
  (params (RunningTime2 :type "Float (double-precision)"))
  (`self.SRV_Move` RunningTime2))

(event `SRV_Move`
  (params (RunningTime2 :type "Float (double-precision)"))
  (set `self.RunningTime2` RunningTime2))

(event `self.Box.OnComponentBeginOverlap`
  (params (OverlappedComponent :type "PrimitiveComponent Object Reference") (OtherActor :type "Actor Object Reference") (OtherComp :type "PrimitiveComponent Object Reference") (OtherBodyIndex :type Integer) (bFromSweep :type Boolean) (SweepResult :type "HitResult Structure (by ref)"))
  (message `/Game/Bishop/INT_Collision.Ragdoll` OtherActor))

(fn `OnRep_ActorTransform`
  (bind _actortransform (`self.ActorTransform`))
  (`KismetSystemLibrary.PrintString` (`KismetStringLibrary.Conv_DoubleToString` (.y (.location _actortransform))) true true (struct :`G` 0.66 :`B` 1.0 :`A` 1.0) 2.0 "1")
  (`self.K2_SetActorLocation` (`KismetMathLibrary.MakeVector` (.x (.location _actortransform)) (.y (.location _actortransform)) (.z (.location _actortransform)))))

(fn `OnRep_RunningTime2`
  (bind _starttransform (`self.StartTransform`))
  (bind _returnvalue (`self.TransformedSin` (`self.RunningTime`)))
  (`self.K2_SetActorLocation` (`KismetMathLibrary.MakeVector` (.x (.location _starttransform)) (+ (.y (.location _starttransform)) _returnvalue) (.z (.location _starttransform)))))

(fn `UserConstructionScript`)