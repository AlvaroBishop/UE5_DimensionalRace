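; Multi-purpose trigger plane that acts as a gravity flipper, ice floor, reset zone or finish for BP_ThirdPersonCharacter_Bishop, chosen by boolean flags in that priority order.
; The construction script sizes the box and plane and sets material and visibility.
; Overlap flips gravity with launch and rotation, lowers friction until exit, restores gravity before respawning, or marks the player first and calls CLFinish on all Bishops.
; The ChangeGravity function is an uncalled force-based variant.
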(event `self.Box.OnComponentBeginOverlap`
  (params (OverlappedComponent :type "PrimitiveComponent Object Reference") (OtherActor :type "Actor Object Reference") (OtherComp :type "PrimitiveComponent Object Reference") (OtherBodyIndex :type Integer) (bFromSweep :type Boolean) (SweepResult :type "HitResult Structure (by ref)"))
  (bind _as_bp_third_person_character_bishop (`self.As BP Third Person Character Bishop`))
  (bind _as_bp_third_person_character_bishop_2 (`self.As BP Third Person Character Bishop`))
  (bind _as_bp_third_person_character_bishop_3 (`self.As BP Third Person Character Bishop`))
  (bind (_returnvalue_roll _returnvalue_pitch _returnvalue_yaw) (`KismetMathLibrary.BreakRotator` (`self.K2_GetActorRotation` _as_bp_third_person_character_bishop)))
  (bind (_returnvalue_roll_2 _returnvalue_pitch_2 _returnvalue_yaw_2) (`KismetMathLibrary.BreakRotator` (`self.K2_GetActorRotation` _as_bp_third_person_character_bishop_3)))
  (bind _charactermovement (`Character.CharacterMovement` (`self.As BP Third Person Character Bishop`)))
  (bind (_returnvalue_x _returnvalue_y _returnvalue_z) (`KismetMathLibrary.BreakVector` (`SceneComponent.K2_GetComponentLocation` (`Character.Mesh` _as_bp_third_person_character_bishop_2))))
  (bind _asbp_third_person_character_bishop (cast `/Game/Bishop/BP_ThirdPersonCharacter_Bishop` OtherActor))
  (set `self.As BP Third Person Character Bishop` _asbp_third_person_character_bishop)
  (if (`self.ChangeGravity?`)
    (if (`/Game/Bishop/BP_ThirdPersonCharacter_Bishop.GravityChanged?` (`self.As BP Third Person Character Bishop`))
      (`Character.LaunchCharacter` (`self.As BP Third Person Character Bishop`) (0.0 0.0 -20.0) false false)
      (`self.K2_SetActorRotation` _as_bp_third_person_character_bishop_3 (`KismetMathLibrary.MakeRotator` _returnvalue_roll_2 180.0 _returnvalue_yaw_2) false)
      (set `CharacterMovementComponent.GravityScale` 1.0 (`Character.CharacterMovement` _as_bp_third_person_character_bishop_3))
      (`PrimitiveComponent.SetLinearDamping` (`Character.CapsuleComponent` (`self.As BP Third Person Character Bishop`)) 0.01)
      (set `/Game/Bishop/BP_ThirdPersonCharacter_Bishop.GravityChanged?` false (`self.As BP Third Person Character Bishop`))
      (else
        (`Character.LaunchCharacter` _as_bp_third_person_character_bishop_2 (0.0 0.0 20.0) false false)
        (`KismetSystemLibrary.Delay` 0.1)
        (`self.K2_TeleportTo` :`self` _as_bp_third_person_character_bishop_2 :`DestLocation` (`KismetMathLibrary.MakeVector` _returnvalue_x _returnvalue_y (+ _returnvalue_z 150.0)))
        (`self.K2_SetActorRotation` _as_bp_third_person_character_bishop (`KismetMathLibrary.MakeRotator` _returnvalue_roll 180.0 _returnvalue_yaw) false)
        (set `CharacterMovementComponent.GravityScale` -1.0 (`Character.CharacterMovement` _as_bp_third_person_character_bishop))
        (`PrimitiveComponent.SetLinearDamping` (`Character.CapsuleComponent` (`self.As BP Third Person Character Bishop`)) 0.01)
        (set `/Game/Bishop/BP_ThirdPersonCharacter_Bishop.GravityChanged?` true (`self.As BP Third Person Character Bishop`))))
    (elif (`self.ItsIce?`)
      (`self.OnIce`)
      (elif (`self.Reset?`)
        (`CharacterMovementComponent.AddForce` _charactermovement (0.0 0.0 300.0))
        (set `CharacterMovementComponent.GravityScale` 1.0 _charactermovement)
        (`PrimitiveComponent.SetLinearDamping` (`Character.CapsuleComponent` (`self.As BP Third Person Character Bishop`)) 0.01)
        (`KismetSystemLibrary.Delay` 0.1)
        (`/Game/Bishop/BP_ThirdPersonCharacter_Bishop.Respawn` (`self.As BP Third Person Character Bishop`))
        (elif (`self.Finish?`)
          (set `/Game/Bishop/BP_ThirdPersonCharacter_Bishop.First?` true (`self.As BP Third Person Character Bishop`))
          (bind _outactors (`GameplayStatics.GetAllActorsOfClass` "/Game/Bishop/BP_ThirdPersonCharacter_Bishop.BP_ThirdPersonCharacter_Bishop_C"))
          (`/Game/Bishop/BP_ThirdPersonCharacter_Bishop.CL_Finish` _outactors))))))

(event `self.Box.OnComponentEndOverlap`
  (params (OverlappedComponent :type "PrimitiveComponent Object Reference") (OtherActor :type "Actor Object Reference") (OtherComp :type "PrimitiveComponent Object Reference") (OtherBodyIndex :type Integer))
  (cast `/Game/Bishop/BP_ThirdPersonCharacter_Bishop` OtherActor)
  (if (`self.ItsIce?`)
    (`self.OutIce`)))

(fn `Change Gravity`
  (bind _as_bp_third_person_character_bishop (`self.As BP Third Person Character Bishop`))
  (bind _as_bp_third_person_character_bishop_2 (`self.As BP Third Person Character Bishop`))
  (bind (_returnvalue_roll _returnvalue_pitch _returnvalue_yaw) (`KismetMathLibrary.BreakRotator` (`self.K2_GetActorRotation` _as_bp_third_person_character_bishop)))
  (bind (_returnvalue_roll_2 _returnvalue_pitch_2 _returnvalue_yaw_2) (`KismetMathLibrary.BreakRotator` (`self.K2_GetActorRotation` _as_bp_third_person_character_bishop_2)))
  (bind _charactermovement (`Character.CharacterMovement` (`self.As BP Third Person Character Bishop`)))
  (bind _charactermovement_2 (`Character.CharacterMovement` (`self.As BP Third Person Character Bishop`)))
  (if (`/Game/Bishop/BP_ThirdPersonCharacter_Bishop.GravityChanged?` (`self.As BP Third Person Character Bishop`))
    (`CharacterMovementComponent.AddForce` _charactermovement (0.0 0.0 300.0))
    (`self.K2_SetActorRotation` _as_bp_third_person_character_bishop_2 (`KismetMathLibrary.MakeRotator` _returnvalue_roll_2 180.0 _returnvalue_yaw_2) false)
    (set `CharacterMovementComponent.GravityScale` 1.0 _charactermovement)
    (`PrimitiveComponent.SetLinearDamping` (`Character.CapsuleComponent` (`self.As BP Third Person Character Bishop`)) 0.01)
    (set `/Game/Bishop/BP_ThirdPersonCharacter_Bishop.GravityChanged?` false (`self.As BP Third Person Character Bishop`))
    (else
      (`CharacterMovementComponent.AddForce` _charactermovement_2 (0.0 0.0 -300.0))
      (`self.K2_SetActorRotation` _as_bp_third_person_character_bishop (`KismetMathLibrary.MakeRotator` _returnvalue_roll 180.0 _returnvalue_yaw) false)
      (set `CharacterMovementComponent.GravityScale` -1.0 _charactermovement_2)
      (`PrimitiveComponent.SetLinearDamping` (`Character.CapsuleComponent` (`self.As BP Third Person Character Bishop`)) 0.01)
      (set `/Game/Bishop/BP_ThirdPersonCharacter_Bishop.GravityChanged?` true (`self.As BP Third Person Character Bishop`)))))

(fn `OnIce`
  (bind _charactermovement (`Character.CharacterMovement` (`self.As BP Third Person Character Bishop`)))
  (set `CharacterMovementComponent.GroundFriction` 0.0 _charactermovement)
  (set `CharacterMovementComponent.BrakingDecelerationWalking` 350.0 _charactermovement))

(fn `OutIce`
  (bind _charactermovement (`Character.CharacterMovement` (`self.As BP Third Person Character Bishop`)))
  (set `CharacterMovementComponent.GroundFriction` 8.0 _charactermovement)
  (set `CharacterMovementComponent.BrakingDecelerationWalking` 2000.0 _charactermovement))

(fn `UserConstructionScript`
  (bind _size (`self.Size`))
  (`SceneComponent.SetVisibility` (`self.Plane`) (`self.ShownPlane`) false)
  (`SceneComponent.SetRelativeScale3D` (`self.Plane`) (`KismetMathLibrary.MakeVector` _size _size 1.0))
  (`SceneComponent.SetRelativeScale3D` (`self.Box`) (`KismetMathLibrary.MakeVector` _size _size 1.0))
  (`PrimitiveComponent.SetMaterial` (`self.Plane`) 0 (`self.Material`)))